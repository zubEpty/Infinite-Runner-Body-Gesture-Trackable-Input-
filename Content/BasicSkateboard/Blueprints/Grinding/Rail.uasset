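; Grindable skateboard rail that carries the player along a spline, with separate gamepad and keyboard character branches.
; The construction script fits a cube and trigger box to the spline length.
; Interaction, or a falling gamepad skater's overlap, starts a speed-scaled timeline, played or reversed by facing dot product; entry-point seeding only affects the gamepad timeline.
; Timeline completion launches the skater using speed and ollie level; JumpOff stops it.
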(event OnComponentBeginOverlap(Box)
  (params (OverlappedComponent :type Primitive%20Component%20Object%20Reference) (OtherActor :type Actor%20Object%20Reference) (OtherComp :type Primitive%20Component%20Object%20Reference) (OtherBodyIndex :type Integer) (bFromSweep :type Boolean) (SweepResult :type Hit%20Result%20Structure%20%28by%20ref%29))
  (bind _returnvalue (Game|GetPlayerCharacter 0))
  (bind _returnvalue_2 (Game|GetPlayerCharacter 0))
  (bind _returnvalue_3 (Game|GetPlayerCharacter 0))
  (bind _returnvalue_4 (Game|GetPlayerCharacter 0))
  (bind _returnvalue_5 (Game|GetPlayerCharacter 0))
  (bind _returnvalue_6 (Game|GetPlayerCharacter 0))
  (bind _spline (Variables|Default|GetSpline))
  (bind _spline_2 (Variables|Default|GetSpline))
  (bind _asskateboard_character_keyboard (Utilities|Casting|CastToSkateboardCharacterKeyboard _returnvalue_2))
  (bind _asskateboard_character_gamepad (Utilities|Casting|CastToSkateboardCharacterGamepad _returnvalue_5))
  (bind _asskateboard_character_gamepad_2 (Utilities|Casting|CastToSkateboardCharacterGamepad _returnvalue))
  (bind _asskateboard_character_gamepad_3 (Utilities|Casting|CastToSkateboardCharacterGamepad _returnvalue_4))
  (bind _asskateboard_character_keyboard_2 (Utilities|Casting|CastToSkateboardCharacterKeyboard _returnvalue_6))
  (bind _asskateboard_character_keyboard_3 (Utilities|Casting|CastToSkateboardCharacterKeyboard _returnvalue_3))
  (bind _returnvalue_7 (Pawn|GetBaseAimRotation _asskateboard_character_keyboard_2))
  (bind _returnvalue_8 (Pawn|GetBaseAimRotation _asskateboard_character_keyboard_2))
  (bind _returnvalue_9 (Pawn|GetBaseAimRotation _asskateboard_character_gamepad_3))
  (bind _returnvalue_10 (Pawn|GetBaseAimRotation _asskateboard_character_gamepad_3))
  (bind _currentspeed (Variables|/Game/BasicSkateboard/Blueprints/SkateboardCharacterGamepad.SkateboardCharacterGamepad_C|GetCurrentSpeed _asskateboard_character_gamepad_3))
  (bind _currentspeed_2 (Variables|/Game/BasicSkateboard/Blueprints/SkateboardCharacterGamepad.SkateboardCharacterGamepad_C|GetCurrentSpeed _asskateboard_character_gamepad_3))
  (bind _currentspeed_3 (Variables|/Game/BasicSkateboard/Blueprints/SkateboardCharacterKeyboard.SkateboardCharacterKeyboard_C|GetCurrentSpeed _asskateboard_character_keyboard_2))
  (bind _currentspeed_4 (Variables|/Game/BasicSkateboard/Blueprints/SkateboardCharacterKeyboard.SkateboardCharacterKeyboard_C|GetCurrentSpeed _asskateboard_character_keyboard_2))
  (bind _returnvalue_11 (Math|Vector|GetForwardVector _returnvalue_7))
  (bind _returnvalue_12 (Math|Vector|GetForwardVector _returnvalue_8))
  (bind _returnvalue_13 (Math|Vector|GetForwardVector _returnvalue_9))
  (bind _returnvalue_14 (Math|Vector|GetForwardVector _returnvalue_10))
  ;[0.5156 0.288 0.1566] Rail Interations
  (bind _asskateboard_character_gamepad_4 (Utilities|Casting|CastToSkateboardCharacterGamepad OtherActor))
  ;;[1 0.1906 0.6203] For Gamepad Character
  (if (Variables|/Game/BasicSkateboard/Blueprints/SkateboardCharacterGamepad.SkateboardCharacterGamepad_C|GetisFalling _asskateboard_character_gamepad_4)
    (Utilities|IsValid _asskateboard_character_gamepad
      (:Is%20Valid
        (Variables|/Game/BasicSkateboard/Blueprints/SkateboardCharacterGamepad.SkateboardCharacterGamepad_C|SetGrinding? _asskateboard_character_gamepad true)
        (CallFunction|GetDistanceRatio)
        (bind _direction (CallFunction|DetectDirection))
        (if (>= _direction 0.0)
          (bind _traveldistance (Timeline|RailTravelGamepad Play)
            (:Update
              (Transformation|SetActorLocation (Game|GetPlayerCharacter 0) (Math|Vector|MakeVector (.x (Spline|GetLocationatDistanceAlongSpline _spline_2 (* _traveldistance (Spline|GetSplineLength _spline_2)) "World")) (.y (Spline|GetLocationatDistanceAlongSpline _spline_2 (* _traveldistance (Spline|GetSplineLength _spline_2)) "World")) (+ (.z (Spline|GetLocationatDistanceAlongSpline _spline_2 (* _traveldistance (Spline|GetSplineLength _spline_2)) "World")) 96.0)) false false))
            (:Finished
              (if (Variables|/Game/BasicSkateboard/Blueprints/SkateboardCharacterGamepad.SkateboardCharacterGamepad_C|GetReversed _asskateboard_character_gamepad_3)
                (Character|LaunchCharacter _asskateboard_character_gamepad_3 (Math|Vector|MakeVector (* (* (* _currentspeed_2 6e+02) (.x _returnvalue_14)) -1.0) (* (* (* _currentspeed_2 6e+02) (.y _returnvalue_14)) -1.0) (+ (* (Math|Conversions|ToFloat(Integer) (Variables|/Game/BasicSkateboard/Blueprints/SkateboardCharacterGamepad.SkateboardCharacterGamepad_C|GetOllieLevel _asskateboard_character_gamepad_3)) 6e+01) 1e+02)) true true)
                (else
                  (Character|LaunchCharacter _asskateboard_character_gamepad_3 (Math|Vector|MakeVector (* (* _currentspeed 6e+02) (.x _returnvalue_13)) (* (* _currentspeed 6e+02) (.y _returnvalue_13)) (+ (* (Math|Conversions|ToFloat(Integer) (Variables|/Game/BasicSkateboard/Blueprints/SkateboardCharacterGamepad.SkateboardCharacterGamepad_C|GetOllieLevel _asskateboard_character_gamepad_3)) 6e+01) 1e+02)) true true)))
              (Variables|/Game/BasicSkateboard/Blueprints/SkateboardCharacterGamepad.SkateboardCharacterGamepad_C|SetIsInAir _asskateboard_character_gamepad_2 true)
              (Variables|/Game/BasicSkateboard/Blueprints/SkateboardCharacterGamepad.SkateboardCharacterGamepad_C|SetGrinding? _asskateboard_character_gamepad_2 false)
              (Variables|/Game/BasicSkateboard/Blueprints/SkateboardCharacterGamepad.SkateboardCharacterGamepad_C|SetOllieLevel _asskateboard_character_gamepad_2 1)))
          (else
            (Timeline|RailTravelGamepad Reverse))))
      (:Is%20Not%20Valid
        ;;[1 0 0.01705] For Keyboard Character
        (Utilities|IsValid _asskateboard_character_keyboard
          (:Is%20Valid
            (Variables|/Game/BasicSkateboard/Blueprints/SkateboardCharacterKeyboard.SkateboardCharacterKeyboard_C|SetGrinding? _asskateboard_character_keyboard true)
            (CallFunction|GetDistanceRatio)
            (bind _direction_2 (CallFunction|DetectDirection))
            (if (>= _direction_2 0.0)
              (bind _traveldistance_2 (Timeline|RailTravelKeyboard Play)
                (:Update
                  (Transformation|SetActorLocation (Game|GetPlayerCharacter 0) (Math|Vector|MakeVector (.x (Spline|GetLocationatDistanceAlongSpline _spline (* _traveldistance_2 (Spline|GetSplineLength _spline)) "World")) (.y (Spline|GetLocationatDistanceAlongSpline _spline (* _traveldistance_2 (Spline|GetSplineLength _spline)) "World")) (+ (.z (Spline|GetLocationatDistanceAlongSpline _spline (* _traveldistance_2 (Spline|GetSplineLength _spline)) "World")) 96.0)) false false))
                (:Finished
                  (if (Variables|/Game/BasicSkateboard/Blueprints/SkateboardCharacterKeyboard.SkateboardCharacterKeyboard_C|GetReversed _asskateboard_character_keyboard_2)
                    (Character|LaunchCharacter _asskateboard_character_keyboard_2 (Math|Vector|MakeVector (* (* (* _currentspeed_3 6e+02) (.x _returnvalue_12)) -1.0) (* (* (* _currentspeed_3 6e+02) (.y _returnvalue_12)) -1.0) (+ (* (Math|Conversions|ToFloat(Integer) (Variables|/Game/BasicSkateboard/Blueprints/SkateboardCharacterKeyboard.SkateboardCharacterKeyboard_C|GetOllieLevel _asskateboard_character_keyboard_2)) 6e+01) 1e+02)) true true)
                    (else
                      (Character|LaunchCharacter _asskateboard_character_keyboard_2 (Math|Vector|MakeVector (* (* _currentspeed_4 6e+02) (.x _returnvalue_11)) (* (* _currentspeed_4 6e+02) (.y _returnvalue_11)) (+ (* (Math|Conversions|ToFloat(Integer) (Variables|/Game/BasicSkateboard/Blueprints/SkateboardCharacterKeyboard.SkateboardCharacterKeyboard_C|GetOllieLevel _asskateboard_character_keyboard_2)) 6e+01) 1e+02)) true true)))
                  (Variables|/Game/BasicSkateboard/Blueprints/SkateboardCharacterKeyboard.SkateboardCharacterKeyboard_C|SetIsInAir _asskateboard_character_keyboard_3 true)
                  (Variables|/Game/BasicSkateboard/Blueprints/SkateboardCharacterKeyboard.SkateboardCharacterKeyboard_C|SetGrinding? _asskateboard_character_keyboard_3 false)
                  (Variables|/Game/BasicSkateboard/Blueprints/SkateboardCharacterKeyboard.SkateboardCharacterKeyboard_C|SetOllieLevel _asskateboard_character_keyboard_3 1)))
              (else
                (Timeline|RailTravelKeyboard Reverse)))))))))

(event EventInteraction
  (bind _returnvalue (Game|GetPlayerCharacter 0))
  (bind _returnvalue_2 (Game|GetPlayerCharacter 0))
  (bind _returnvalue_3 (Game|GetPlayerCharacter 0))
  (bind _returnvalue_4 (Game|GetPlayerCharacter 0))
  (bind _returnvalue_5 (Game|GetPlayerCharacter 0))
  (bind _returnvalue_6 (Game|GetPlayerCharacter 0))
  (bind _spline (Variables|Default|GetSpline))
  (bind _spline_2 (Variables|Default|GetSpline))
  (bind _asskateboard_character_keyboard (Utilities|Casting|CastToSkateboardCharacterKeyboard _returnvalue_2))
  (bind _asskateboard_character_gamepad (Utilities|Casting|CastToSkateboardCharacterGamepad _returnvalue_5))
  (bind _asskateboard_character_gamepad_2 (Utilities|Casting|CastToSkateboardCharacterGamepad _returnvalue))
  (bind _asskateboard_character_gamepad_3 (Utilities|Casting|CastToSkateboardCharacterGamepad _returnvalue_4))
  (bind _asskateboard_character_keyboard_2 (Utilities|Casting|CastToSkateboardCharacterKeyboard _returnvalue_6))
  (bind _asskateboard_character_keyboard_3 (Utilities|Casting|CastToSkateboardCharacterKeyboard _returnvalue_3))
  (bind _returnvalue_7 (Pawn|GetBaseAimRotation _asskateboard_character_keyboard_2))
  (bind _returnvalue_8 (Pawn|GetBaseAimRotation _asskateboard_character_keyboard_2))
  (bind _returnvalue_9 (Pawn|GetBaseAimRotation _asskateboard_character_gamepad_3))
  (bind _returnvalue_10 (Pawn|GetBaseAimRotation _asskateboard_character_gamepad_3))
  (bind _currentspeed (Variables|/Game/BasicSkateboard/Blueprints/SkateboardCharacterGamepad.SkateboardCharacterGamepad_C|GetCurrentSpeed _asskateboard_character_gamepad_3))
  (bind _currentspeed_2 (Variables|/Game/BasicSkateboard/Blueprints/SkateboardCharacterGamepad.SkateboardCharacterGamepad_C|GetCurrentSpeed _asskateboard_character_gamepad_3))
  (bind _currentspeed_3 (Variables|/Game/BasicSkateboard/Blueprints/SkateboardCharacterKeyboard.SkateboardCharacterKeyboard_C|GetCurrentSpeed _asskateboard_character_keyboard_2))
  (bind _currentspeed_4 (Variables|/Game/BasicSkateboard/Blueprints/SkateboardCharacterKeyboard.SkateboardCharacterKeyboard_C|GetCurrentSpeed _asskateboard_character_keyboard_2))
  (bind _returnvalue_11 (Math|Vector|GetForwardVector _returnvalue_7))
  (bind _returnvalue_12 (Math|Vector|GetForwardVector _returnvalue_8))
  (bind _returnvalue_13 (Math|Vector|GetForwardVector _returnvalue_9))
  (bind _returnvalue_14 (Math|Vector|GetForwardVector _returnvalue_10))
  ;[0.5156 0.288 0.1566] Rail Interations
  ;;[1 0.1906 0.6203] For Gamepad Character
  (Utilities|IsValid _asskateboard_character_gamepad
    (:Is%20Valid
      (Variables|/Game/BasicSkateboard/Blueprints/SkateboardCharacterGamepad.SkateboardCharacterGamepad_C|SetGrinding? _asskateboard_character_gamepad true)
      (CallFunction|GetDistanceRatio)
      (bind _direction (CallFunction|DetectDirection))
      (if (>= _direction 0.0)
        (bind _traveldistance (Timeline|RailTravelGamepad Play)
          (:Update
            (Transformation|SetActorLocation (Game|GetPlayerCharacter 0) (Math|Vector|MakeVector (.x (Spline|GetLocationatDistanceAlongSpline _spline_2 (* _traveldistance (Spline|GetSplineLength _spline_2)) "World")) (.y (Spline|GetLocationatDistanceAlongSpline _spline_2 (* _traveldistance (Spline|GetSplineLength _spline_2)) "World")) (+ (.z (Spline|GetLocationatDistanceAlongSpline _spline_2 (* _traveldistance (Spline|GetSplineLength _spline_2)) "World")) 96.0)) false false))
          (:Finished
            (if (Variables|/Game/BasicSkateboard/Blueprints/SkateboardCharacterGamepad.SkateboardCharacterGamepad_C|GetReversed _asskateboard_character_gamepad_3)
              (Character|LaunchCharacter _asskateboard_character_gamepad_3 (Math|Vector|MakeVector (* (* (* _currentspeed_2 6e+02) (.x _returnvalue_14)) -1.0) (* (* (* _currentspeed_2 6e+02) (.y _returnvalue_14)) -1.0) (+ (* (Math|Conversions|ToFloat(Integer) (Variables|/Game/BasicSkateboard/Blueprints/SkateboardCharacterGamepad.SkateboardCharacterGamepad_C|GetOllieLevel _asskateboard_character_gamepad_3)) 6e+01) 1e+02)) true true)
              (else
                (Character|LaunchCharacter _asskateboard_character_gamepad_3 (Math|Vector|MakeVector (* (* _currentspeed 6e+02) (.x _returnvalue_13)) (* (* _currentspeed 6e+02) (.y _returnvalue_13)) (+ (* (Math|Conversions|ToFloat(Integer) (Variables|/Game/BasicSkateboard/Blueprints/SkateboardCharacterGamepad.SkateboardCharacterGamepad_C|GetOllieLevel _asskateboard_character_gamepad_3)) 6e+01) 1e+02)) true true)))
            (Variables|/Game/BasicSkateboard/Blueprints/SkateboardCharacterGamepad.SkateboardCharacterGamepad_C|SetIsInAir _asskateboard_character_gamepad_2 true)
            (Variables|/Game/BasicSkateboard/Blueprints/SkateboardCharacterGamepad.SkateboardCharacterGamepad_C|SetGrinding? _asskateboard_character_gamepad_2 false)
            (Variables|/Game/BasicSkateboard/Blueprints/SkateboardCharacterGamepad.SkateboardCharacterGamepad_C|SetOllieLevel _asskateboard_character_gamepad_2 1)))
        (else
          (Timeline|RailTravelGamepad Reverse))))
    (:Is%20Not%20Valid
      ;;[1 0 0.01705] For Keyboard Character
      (Utilities|IsValid _asskateboard_character_keyboard
        (:Is%20Valid
          (Variables|/Game/BasicSkateboard/Blueprints/SkateboardCharacterKeyboard.SkateboardCharacterKeyboard_C|SetGrinding? _asskateboard_character_keyboard true)
          (CallFunction|GetDistanceRatio)
          (bind _direction_2 (CallFunction|DetectDirection))
          (if (>= _direction_2 0.0)
            (bind _traveldistance_2 (Timeline|RailTravelKeyboard Play)
              (:Update
                (Transformation|SetActorLocation (Game|GetPlayerCharacter 0) (Math|Vector|MakeVector (.x (Spline|GetLocationatDistanceAlongSpline _spline (* _traveldistance_2 (Spline|GetSplineLength _spline)) "World")) (.y (Spline|GetLocationatDistanceAlongSpline _spline (* _traveldistance_2 (Spline|GetSplineLength _spline)) "World")) (+ (.z (Spline|GetLocationatDistanceAlongSpline _spline (* _traveldistance_2 (Spline|GetSplineLength _spline)) "World")) 96.0)) false false))
              (:Finished
                (if (Variables|/Game/BasicSkateboard/Blueprints/SkateboardCharacterKeyboard.SkateboardCharacterKeyboard_C|GetReversed _asskateboard_character_keyboard_2)
                  (Character|LaunchCharacter _asskateboard_character_keyboard_2 (Math|Vector|MakeVector (* (* (* _currentspeed_3 6e+02) (.x _returnvalue_12)) -1.0) (* (* (* _currentspeed_3 6e+02) (.y _returnvalue_12)) -1.0) (+ (* (Math|Conversions|ToFloat(Integer) (Variables|/Game/BasicSkateboard/Blueprints/SkateboardCharacterKeyboard.SkateboardCharacterKeyboard_C|GetOllieLevel _asskateboard_character_keyboard_2)) 6e+01) 1e+02)) true true)
                  (else
                    (Character|LaunchCharacter _asskateboard_character_keyboard_2 (Math|Vector|MakeVector (* (* _currentspeed_4 6e+02) (.x _returnvalue_11)) (* (* _currentspeed_4 6e+02) (.y _returnvalue_11)) (+ (* (Math|Conversions|ToFloat(Integer) (Variables|/Game/BasicSkateboard/Blueprints/SkateboardCharacterKeyboard.SkateboardCharacterKeyboard_C|GetOllieLevel _asskateboard_character_keyboard_2)) 6e+01) 1e+02)) true true)))
                (Variables|/Game/BasicSkateboard/Blueprints/SkateboardCharacterKeyboard.SkateboardCharacterKeyboard_C|SetIsInAir _asskateboard_character_keyboard_3 true)
                (Variables|/Game/BasicSkateboard/Blueprints/SkateboardCharacterKeyboard.SkateboardCharacterKeyboard_C|SetGrinding? _asskateboard_character_keyboard_3 false)
                (Variables|/Game/BasicSkateboard/Blueprints/SkateboardCharacterKeyboard.SkateboardCharacterKeyboard_C|SetOllieLevel _asskateboard_character_keyboard_3 1)))
            (else
              (Timeline|RailTravelKeyboard Reverse))))))))

(event EventTick
  (params (DeltaSeconds :type Float%20%28single-precision%29))
  (bind _returnvalue (Game|GetPlayerCharacter 0))
  (bind _returnvalue_2 (Game|GetPlayerCharacter 0))
  (bind _asskateboard_character_gamepad (Utilities|Casting|CastToSkateboardCharacterGamepad _returnvalue))
  (bind _asskateboard_character_keyboard (Utilities|Casting|CastToSkateboardCharacterKeyboard _returnvalue_2))
  ;[1 0.1906 0.6203] Match Rail Grind Speed to Player Speed Gamepad Character
  (Utilities|IsValid _asskateboard_character_gamepad
    (:Is%20Valid
      (Components|Timeline|SetPlayRate (Variables|Default|GetRailTravelGamepad) (/ (Variables|/Game/BasicSkateboard/Blueprints/SkateboardCharacterGamepad.SkateboardCharacterGamepad_C|GetCurrentSpeed _asskateboard_character_gamepad) (/ (Spline|GetSplineLength (Variables|Default|GetSpline)) 1e+03))))
    (:Is%20Not%20Valid
      ;[1 0 0.01705] Match rail grind speed to player speed Keyboard Character
      (Utilities|IsValid _asskateboard_character_keyboard
        (:Is%20Valid
          (Components|Timeline|SetPlayRate (Variables|Default|GetRailTravelKeyboard) (/ (Variables|/Game/BasicSkateboard/Blueprints/SkateboardCharacterKeyboard.SkateboardCharacterKeyboard_C|GetCurrentSpeed _asskateboard_character_keyboard) (/ (Spline|GetSplineLength (Variables|Default|GetSpline)) 1e+03))))))))

(event EventJumpOff
  (bind _returnvalue (Game|GetPlayerCharacter 0))
  (bind _returnvalue_2 (Game|GetPlayerCharacter 0))
  (bind _returnvalue_3 (Game|GetPlayerCharacter 0))
  (bind _returnvalue_4 (Game|GetPlayerCharacter 0))
  (bind _spline (Variables|Default|GetSpline))
  (bind _spline_2 (Variables|Default|GetSpline))
  (bind _asskateboard_character_gamepad (Utilities|Casting|CastToSkateboardCharacterGamepad _returnvalue))
  (bind _asskateboard_character_gamepad_2 (Utilities|Casting|CastToSkateboardCharacterGamepad _returnvalue_3))
  (bind _asskateboard_character_keyboard (Utilities|Casting|CastToSkateboardCharacterKeyboard _returnvalue_4))
  (bind _asskateboard_character_keyboard_2 (Utilities|Casting|CastToSkateboardCharacterKeyboard _returnvalue_2))
  (bind _returnvalue_5 (Pawn|GetBaseAimRotation _asskateboard_character_keyboard))
  (bind _returnvalue_6 (Pawn|GetBaseAimRotation _asskateboard_character_keyboard))
  (bind _returnvalue_7 (Pawn|GetBaseAimRotation _asskateboard_character_gamepad_2))
  (bind _returnvalue_8 (Pawn|GetBaseAimRotation _asskateboard_character_gamepad_2))
  (bind _currentspeed (Variables|/Game/BasicSkateboard/Blueprints/SkateboardCharacterGamepad.SkateboardCharacterGamepad_C|GetCurrentSpeed _asskateboard_character_gamepad_2))
  (bind _currentspeed_2 (Variables|/Game/BasicSkateboard/Blueprints/SkateboardCharacterGamepad.SkateboardCharacterGamepad_C|GetCurrentSpeed _asskateboard_character_gamepad_2))
  (bind _currentspeed_3 (Variables|/Game/BasicSkateboard/Blueprints/SkateboardCharacterKeyboard.SkateboardCharacterKeyboard_C|GetCurrentSpeed _asskateboard_character_keyboard))
  (bind _currentspeed_4 (Variables|/Game/BasicSkateboard/Blueprints/SkateboardCharacterKeyboard.SkateboardCharacterKeyboard_C|GetCurrentSpeed _asskateboard_character_keyboard))
  (bind _returnvalue_9 (Math|Vector|GetForwardVector _returnvalue_5))
  (bind _returnvalue_10 (Math|Vector|GetForwardVector _returnvalue_6))
  (bind _returnvalue_11 (Math|Vector|GetForwardVector _returnvalue_7))
  (bind _returnvalue_12 (Math|Vector|GetForwardVector _returnvalue_8))
  ;[0.5156 0.288 0.1566] Rail Interations
  (Utilities|IsValid (.AsSkateboard%20Character%20Gamepad (Utilities|Casting|CastToSkateboardCharacterGamepad (Game|GetPlayerCharacter 0)))
    (:Is%20Valid
      ;;[1 0.1906 0.6203] For Gamepad Character
      (bind _traveldistance (Timeline|RailTravelGamepad Stop)
        (:Update
          (Transformation|SetActorLocation (Game|GetPlayerCharacter 0) (Math|Vector|MakeVector (.x (Spline|GetLocationatDistanceAlongSpline _spline_2 (* _traveldistance (Spline|GetSplineLength _spline_2)) "World")) (.y (Spline|GetLocationatDistanceAlongSpline _spline_2 (* _traveldistance (Spline|GetSplineLength _spline_2)) "World")) (+ (.z (Spline|GetLocationatDistanceAlongSpline _spline_2 (* _traveldistance (Spline|GetSplineLength _spline_2)) "World")) 96.0)) false false))
        (:Finished
          (if (Variables|/Game/BasicSkateboard/Blueprints/SkateboardCharacterGamepad.SkateboardCharacterGamepad_C|GetReversed _asskateboard_character_gamepad_2)
            (Character|LaunchCharacter _asskateboard_character_gamepad_2 (Math|Vector|MakeVector (* (* (* _currentspeed_2 6e+02) (.x _returnvalue_12)) -1.0) (* (* (* _currentspeed_2 6e+02) (.y _returnvalue_12)) -1.0) (+ (* (Math|Conversions|ToFloat(Integer) (Variables|/Game/BasicSkateboard/Blueprints/SkateboardCharacterGamepad.SkateboardCharacterGamepad_C|GetOllieLevel _asskateboard_character_gamepad_2)) 6e+01) 1e+02)) true true)
            (else
              (Character|LaunchCharacter _asskateboard_character_gamepad_2 (Math|Vector|MakeVector (* (* _currentspeed 6e+02) (.x _returnvalue_11)) (* (* _currentspeed 6e+02) (.y _returnvalue_11)) (+ (* (Math|Conversions|ToFloat(Integer) (Variables|/Game/BasicSkateboard/Blueprints/SkateboardCharacterGamepad.SkateboardCharacterGamepad_C|GetOllieLevel _asskateboard_character_gamepad_2)) 6e+01) 1e+02)) true true)))
          (Variables|/Game/BasicSkateboard/Blueprints/SkateboardCharacterGamepad.SkateboardCharacterGamepad_C|SetIsInAir _asskateboard_character_gamepad true)
          (Variables|/Game/BasicSkateboard/Blueprints/SkateboardCharacterGamepad.SkateboardCharacterGamepad_C|SetGrinding? _asskateboard_character_gamepad false)
          (Variables|/Game/BasicSkateboard/Blueprints/SkateboardCharacterGamepad.SkateboardCharacterGamepad_C|SetOllieLevel _asskateboard_character_gamepad 1))))
    (:Is%20Not%20Valid
      ;;[1 0 0.01705] For Keyboard Character
      (bind _traveldistance_2 (Timeline|RailTravelKeyboard Stop)
        (:Update
          (Transformation|SetActorLocation (Game|GetPlayerCharacter 0) (Math|Vector|MakeVector (.x (Spline|GetLocationatDistanceAlongSpline _spline (* _traveldistance_2 (Spline|GetSplineLength _spline)) "World")) (.y (Spline|GetLocationatDistanceAlongSpline _spline (* _traveldistance_2 (Spline|GetSplineLength _spline)) "World")) (+ (.z (Spline|GetLocationatDistanceAlongSpline _spline (* _traveldistance_2 (Spline|GetSplineLength _spline)) "World")) 96.0)) false false))
        (:Finished
          (if (Variables|/Game/BasicSkateboard/Blueprints/SkateboardCharacterKeyboard.SkateboardCharacterKeyboard_C|GetReversed _asskateboard_character_keyboard)
            (Character|LaunchCharacter _asskateboard_character_keyboard (Math|Vector|MakeVector (* (* (* _currentspeed_3 6e+02) (.x _returnvalue_10)) -1.0) (* (* (* _currentspeed_3 6e+02) (.y _returnvalue_10)) -1.0) (+ (* (Math|Conversions|ToFloat(Integer) (Variables|/Game/BasicSkateboard/Blueprints/SkateboardCharacterKeyboard.SkateboardCharacterKeyboard_C|GetOllieLevel _asskateboard_character_keyboard)) 6e+01) 1e+02)) true true)
            (else
              (Character|LaunchCharacter _asskateboard_character_keyboard (Math|Vector|MakeVector (* (* _currentspeed_4 6e+02) (.x _returnvalue_9)) (* (* _currentspeed_4 6e+02) (.y _returnvalue_9)) (+ (* (Math|Conversions|ToFloat(Integer) (Variables|/Game/BasicSkateboard/Blueprints/SkateboardCharacterKeyboard.SkateboardCharacterKeyboard_C|GetOllieLevel _asskateboard_character_keyboard)) 6e+01) 1e+02)) true true)))
          (Variables|/Game/BasicSkateboard/Blueprints/SkateboardCharacterKeyboard.SkateboardCharacterKeyboard_C|SetIsInAir _asskateboard_character_keyboard_2 true)
          (Variables|/Game/BasicSkateboard/Blueprints/SkateboardCharacterKeyboard.SkateboardCharacterKeyboard_C|SetGrinding? _asskateboard_character_keyboard_2 false)
          (Variables|/Game/BasicSkateboard/Blueprints/SkateboardCharacterKeyboard.SkateboardCharacterKeyboard_C|SetOllieLevel _asskateboard_character_keyboard_2 1))))))

(fn ConstructionScript
  (CallFunction|ConstructRail)
  (CallFunction|ConstructCollision))

(fn ConstructRail
  (Transformation|SetWorldScale3D (Variables|Default|GetCube) (Math|Vector|MakeVector (* (Spline|GetSplineLength (Variables|Default|GetSpline)) 0.01) 0.1 0.1)))

(fn ConstructCollision
  (bind _box (Variables|Default|GetBox))
  (bind _output_get (LocalVariables|SetHalfLength_L (/ (Spline|GetSplineLength (Variables|Default|GetSpline)) 2.0)))
  (Components|Box|SetBoxExtent _box (Math|Vector|MakeVector 6.0 6.0 _output_get) true)
  (Transformation|SetWorldTransform _box (Math|Transform|MakeTransform (.location (Spline|GetTransformatDistanceAlongSpline (Variables|Default|GetSpline) (LocalVariables|GetHalfLength_L) "World" false)) (Math|Rotator|MakeRotator (.roll (.rotation (Spline|GetTransformatDistanceAlongSpline (Variables|Default|GetSpline) (LocalVariables|GetHalfLength_L) "World" false))) (+ (.pitch (.rotation (Spline|GetTransformatDistanceAlongSpline (Variables|Default|GetSpline) (LocalVariables|GetHalfLength_L) "World" false))) 9e+01) (.yaw (.rotation (Spline|GetTransformatDistanceAlongSpline (Variables|Default|GetSpline) (LocalVariables|GetHalfLength_L) "World" false)))) "1,1,1") false false))

(fn DetectDirection
  (bind _returnvalue (Game|GetPlayerCharacter 0))
  (bind _arrow (Variables|Default|GetArrow))
  (bind _arrow_2 (Variables|Default|GetArrow))
  (bind _returnvalue_2 (Transformation|GetWorldRotation _arrow))
  (bind _returnvalue_3 (Transformation|GetWorldRotation _arrow_2))
  (Utilities|IsValid (.AsSkateboard%20Character%20Gamepad (Utilities|Casting|CastToSkateboardCharacterGamepad (Game|GetPlayerCharacter 0)))
    (:Is%20Valid
      ;[1 1 1] Gamepad Character
      (if (Variables|/Game/BasicSkateboard/Blueprints/SkateboardCharacterGamepad.SkateboardCharacterGamepad_C|GetReversed (.AsSkateboard%20Character%20Gamepad (Utilities|Casting|CastToSkateboardCharacterGamepad (Game|GetPlayerCharacter 0))))
        (return (Math|Vector|DotProduct (Math|Vector|GetForwardVector (Pawn|GetBaseAimRotation (Game|GetPlayerCharacter 0))) (Math|Vector|GetForwardVector (Math|Rotator|MakeRotator (* (.roll _returnvalue_3) -1.0) (* (.pitch _returnvalue_3) -1.0) (* (.yaw _returnvalue_3) -1.0)))))
        (else
          (return (Math|Vector|DotProduct (Math|Vector|GetForwardVector (Pawn|GetBaseAimRotation (Game|GetPlayerCharacter 0))) (Math|Vector|GetForwardVector (Transformation|GetWorldRotation (Variables|Default|GetArrow))))))))
    (:Is%20Not%20Valid
      ;[1 1 1] Keyboard Character
      (if (Variables|/Game/BasicSkateboard/Blueprints/SkateboardCharacterKeyboard.SkateboardCharacterKeyboard_C|GetReversed (.AsSkateboard%20Character%20Keyboard (Utilities|Casting|CastToSkateboardCharacterKeyboard _returnvalue)))
        (return (Math|Vector|DotProduct (Math|Vector|GetForwardVector (Pawn|GetBaseAimRotation (Game|GetPlayerCharacter 0))) (Math|Vector|GetForwardVector (Math|Rotator|MakeRotator (* (.roll _returnvalue_2) -1.0) (* (.pitch _returnvalue_2) -1.0) (* (.yaw _returnvalue_2) -1.0)))))
        (else
          (return (Math|Vector|DotProduct (Math|Vector|GetForwardVector (Pawn|GetBaseAimRotation _returnvalue)) (Math|Vector|GetForwardVector (Transformation|GetWorldRotation (Variables|Default|GetArrow))))))))))

(fn GetDistanceRatio
  (bind _railtravelgamepad (Variables|Default|GetRailTravelGamepad))
  (Components|Timeline|SetNewTime _railtravelgamepad (* (Components|Timeline|GetTimelineLength _railtravelgamepad) (/ (Math|Vector|VectorLength (- (Transformation|GetActorLocation (Game|GetPlayerCharacter 0)) (Spline|GetLocationatSplinePoint (Variables|Default|GetSpline) 0 "World"))) (Spline|GetSplineLength (Variables|Default|GetSpline))))))