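; Letter actor for the skateboard game that displays a configurable letter and spins continuously in the world.
; On BeginPlay it writes the Letter value to two text render components and stores the initial rotation of LetterCollision.
; A looping LetterSpin timeline adds its track value to the starting yaw and restarts whenever it finishes.
; The graph contains no overlap or pickup logic.
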(event EventBeginPlay
  (bind _output_get (Variables|Default|SetLetter (Variables|Default|GetLetter)))
  (Rendering|Components|TextRender|SetText (Variables|Default|GetTextRender) (Utilities|Text|ToText(String) _output_get))
  (Rendering|Components|TextRender|SetText (Variables|Default|GetTextRender1) (Utilities|Text|ToText(String) _output_get))
  (Variables|Default|SetInitialRotaion (Transformation|GetWorldRotation (Variables|Default|GetLetterCollision)))
  (bind _newtrack_0 (Timeline|Letter%20Spin Play)
    (:Update
      (Transformation|SetWorldRotation (Variables|Default|GetLetterCollision) (Math|Rotator|MakeRotator (.roll (Variables|Default|GetInitialRotaion)) (.pitch (Variables|Default|GetInitialRotaion)) (+ _newtrack_0 (.yaw (Variables|Default|GetInitialRotaion)))) false false))
    (:Finished
      (Timeline|Letter%20Spin PlayFromStart))))

(event Collision|EventActorBeginOverlap
  (params (OtherActor :type Actor%20Object%20Reference)))

(event EventTick
  (params (DeltaSeconds :type Float%20%28single-precision%29)))

(fn ConstructionScript)