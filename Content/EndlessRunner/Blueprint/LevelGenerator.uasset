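; LevelGenerator is an endless-runner actor that builds the track and shows the run HUD.
; On BeginPlay it adds WBP_RunHUD to the viewport and pre-spawns a batch of tiles through AddTile.
; AddTile spawns a random class from FloorTiles at NewSpawnPoint, then takes that BP_SkateTile's attach transform as the next spawn point, chaining tiles end to end.
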(event EventBeginPlay
  (bind _returnvalue (UserInterface|CreateWidget "/Game/EndlessRunner/UMG/WBP_RunHUD.WBP_RunHUD_C"))
  (UserInterface|Viewport|AddtoViewport _returnvalue 0)
  (for _index (range 0 9)
    (CallFunction|AddTile)))

(event Collision|EventActorBeginOverlap
  (params (OtherActor :type Actor%20Object%20Reference)))

(event EventTick
  (params (DeltaSeconds :type Float%20%28single-precision%29)))

(fn ConstructionScript)

(fn AddTile
  (bind _floortiles (Variables|Default|GetFloorTiles))
  (bind _returnvalue (Game|SpawnActorfromClass (Utilities|Array|Get(acopy) _floortiles (Math|Random|RandomIntegerinRange 0 (Utilities|Array|LastIndex _floortiles))) (Variables|Default|GetNewSpawnPoint) "Undefined" 0 0))
  (bind _asbp_skate_tile (Utilities|Casting|CastToBP_SkateTile _returnvalue))
  (bind _attachtransform (Default|GetAttachTransform _asbp_skate_tile))
  (Variables|Default|SetNewSpawnPoint _attachtransform))